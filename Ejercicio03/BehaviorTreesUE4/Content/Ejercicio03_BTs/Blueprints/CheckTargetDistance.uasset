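; CheckTargetDistance is a Behavior Tree decorator that passes when the AI's pawn is close enough to the target it follows.
; It reads the target actor from the TargetToFollow blackboard key and casts the owner to MyAIController, storing that reference to reach the controlled pawn.
; The check compares the straight-line distance between both actors against AcceptableDistance, failing if the target is invalid or the cast fails.
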(fn `PerformConditionCheck`
  (params (OwnerActor :type "Actor Object Reference"))
  (returns (ReturnValue :type Boolean))
  (bind _returnvalue (`BTFunctionLibrary.GetBlackboardValueAsActor` (`self.TargetToFollow`)))
  (`/Engine/EditorBlueprintResources/StandardMacros.IsValid` _returnvalue
    (:`Is Valid`
      (bind _asmy_aicontroller (cast `/Game/Ejercicio03_BTs/Blueprints/MyAIController` OwnerActor)
        (:`then`
          (set `self.AICtrlRef` _asmy_aicontroller)
          (return (<= (`KismetMathLibrary.VSize` (- (`Actor.K2_GetActorLocation` _returnvalue) (`Actor.K2_GetActorLocation` (`Controller.K2_GetPawn` (`self.AICtrlRef`))))) (`self.AcceptableDistance`))))
        (:`CastFailed`
          _)))
    (:`Is Not Valid`
      _))
  (return false))
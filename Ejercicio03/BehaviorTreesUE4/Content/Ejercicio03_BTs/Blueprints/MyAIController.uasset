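; AI controller for an AI character that runs a behavior tree and switches between patrol and chase movement speeds.
; On BeginPlay it initializes its blackboard, seeds WaypointLocation with the pawn's current location and starts the tree.
; An UpdatePawnSpeed event casts the pawn to AI_Character and sets its MaxWalkSpeed from the requested speed mode.
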(event `self.ReceiveBeginPlay`
  (`self.UseBlackboard` "/Game/Ejercicio03_BTs/Blueprints/MyBlackboard.MyBlackboard")
  (`BlackboardComponent.SetValueAsVector` (`AIBlueprintHelperLibrary.GetBlackboard` self) (`self.WaypointLocation`) (`self.K2_GetActorLocation` (`self.K2_GetPawn`)))
  (`self.RunBehaviorTree` "/Game/Ejercicio03_BTs/Blueprints/MyBehaviorTree.MyBehaviorTree"))

(event `UpdatePawnSpeed`
  (params (Speed :type "/Game/Ejercicio03_BTs/Blueprints/SpeedSelector Enum" :default "NewEnumerator0"))
  (bind _asai_character (cast `/Game/Ejercicio03_BTs/Blueprints/AI_Character` (`self.K2_GetPawn`)))
  (switch `/Game/Ejercicio03_BTs/Blueprints/SpeedSelector` Speed
    (:`NewEnumerator0`
      (bind _charactermovement (`Character.CharacterMovement` _asai_character))
      (set `CharacterMovementComponent.MaxWalkSpeed` (`self.PatrolSpeed`) _charactermovement))
    (:`NewEnumerator1`
      (set `CharacterMovementComponent.MaxWalkSpeed` (`self.ChaseSpeed`) _charactermovement))))

(fn `UserConstructionScript`)
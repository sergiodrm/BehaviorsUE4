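; Behavior Tree service that advances an AI character through the waypoints of its route.
; While active, it binds to the MyAIController move-completed event, then unbinds and clears the cached controller on deactivation.
; Each successful move increments the Blackboard route index, wrapping around the AI_Character's Route array, and writes that waypoint actor's location to the Blackboard.
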(event `self.ReceiveActivation`
  (params (OwnerActor :type "Actor Object Reference"))
  (bind _asmy_aicontroller (cast `/Game/Ejercicio03_BTs/Blueprints/MyAIController` OwnerActor))
  (add `AIController.ReceiveMoveCompleted` _asmy_aicontroller (delegate `CustomEvent_0`))
  (set `self.AICtrlRef` _asmy_aicontroller))

(event `self.ReceiveDeactivation`
  (params (OwnerActor :type "Actor Object Reference"))
  (bind _asmy_aicontroller (cast `/Game/Ejercicio03_BTs/Blueprints/MyAIController` OwnerActor))
  (remove `AIController.ReceiveMoveCompleted` _asmy_aicontroller (delegate `CustomEvent_0`))
  (set `self.AICtrlRef` null))

(event `CustomEvent_0`
  (params (RequestID :type "AIRequestID Structure") (Result :type "EPathFollowingResult Enum" :default "Success"))
  (switch `EPathFollowingResult` Result
    (:`Success`
      (bind _asai_character (cast `/Game/Ejercicio03_BTs/Blueprints/AI_Character` (`Controller.K2_GetPawn` (`self.AICtrlRef`))))
      (bind _route (`/Game/Ejercicio03_BTs/Blueprints/AI_Character.Route` _asai_character))
      (`BTFunctionLibrary.SetBlackboardValueAsInt` (`self.RouteIdxKey`) (mod (+ (`BTFunctionLibrary.GetBlackboardValueAsInt` (`self.RouteIdxKey`)) 1) (`KismetArrayLibrary.Array_Length` _route)))
      (`BTFunctionLibrary.SetBlackboardValueAsVector` (`self.WaypointLocation`) (`Actor.K2_GetActorLocation` (`|GetArrayItem` _route (`BTFunctionLibrary.GetBlackboardValueAsInt` (`self.RouteIdxKey`))))))))
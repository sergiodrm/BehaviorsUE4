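; TargetSearch is a Behavior Tree node that looks for a visible target around the AI pawn on each tick.
; A sphere trace gathers nearby objects, ignoring AI characters, then line traces confirm sight.
; A visible hit updates blackboard target and location and changes pawn speed; new targets must also be within AcceptableDistance.
; Failed checks clear TargetToFollow but leave the last TargetLocation intact.
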(event `self.ReceiveTickAI`
  (params (OwnerController :type "AIController Object Reference") (ControlledPawn :type "Pawn Object Reference") (DeltaSeconds :type "Float (single-precision)"))
  (if (not (!= (`self.AICtrlRef`) null))
    (bind _asmy_aicontroller (cast `/Game/Ejercicio03_BTs/Blueprints/MyAIController` OwnerController))
    (set `self.AICtrlRef` _asmy_aicontroller))
  (bind _output_get (set `self.MyLocation` (`Actor.K2_GetActorLocation` (`Controller.K2_GetPawn` (`self.AICtrlRef`)))))
  (bind _outactors (`GameplayStatics.GetAllActorsOfClass` "/Game/Ejercicio03_BTs/Blueprints/AI_Character.AI_Character_C"))
  (bind _outhits (`KismetSystemLibrary.SphereTraceMultiForObjects` _output_get (+ _output_get (0.0 0.0 15.0)) 1500.0 (`self.DesiredObjectTypes`) false _outactors))
  (for _array_element _outhits
    (bind (_bblockinghit _binitialoverlap _time _distance _location _impactpoint _normal _impactnormal _physmat _hitactor) (`GameplayStatics.BreakHitResult` _array_element))
    (bind _outhit (`KismetSystemLibrary.LineTraceSingle` (`self.MyLocation`) (`Actor.K2_GetActorLocation` _hitactor) "TraceTypeQuery2" false _outactors))
    (bind (_bblockinghit_2 _binitialoverlap_2 _time_2 _distance_2 _location_2 _impactpoint_2 _normal_2 _impactnormal_2 _physmat_2 _hitactor_2) (`GameplayStatics.BreakHitResult` _outhit))
    (if (== _hitactor_2 _hitactor)
      (if (!= (`BTFunctionLibrary.GetBlackboardValueAsActor` (`self.TargetToFollow`)) null)
        (`BTFunctionLibrary.SetBlackboardValueAsObject` (`self.TargetToFollow`) _hitactor_2 :!label _label)
        (`BTFunctionLibrary.SetBlackboardValueAsVector` (`self.TargetLocation`) (`Actor.K2_GetActorLocation` _hitactor_2))
        (`BTFunctionLibrary.SetBlackboardValueAsBool` (`self.TargetLocationValid`) true)
        (`/Game/Ejercicio03_BTs/Blueprints/MyAIController.UpdatePawnSpeed` (`self.AICtrlRef`) "NewEnumerator1")
        (break)
        (elif (<= (`KismetMathLibrary.VSize` (- (`Actor.K2_GetActorLocation` (`Controller.K2_GetPawn` (`self.AICtrlRef`))) (`Actor.K2_GetActorLocation` _hitactor_2))) (`self.AcceptableDistance`))
          (goto _label)
          (else
            (`BTFunctionLibrary.SetBlackboardValueAsObject` (`self.TargetToFollow`)))))
      (else
        (`BTFunctionLibrary.SetBlackboardValueAsObject` (`self.TargetToFollow`))))))